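; PowerupBlockBP is a sprite-based block that bumps when an airborne Character overlaps it, with only a debug print and no powerup logic yet.
; Any Character overlap disables collision; if falling and not already hit, a timeline lerps BlockSprite along local Z.
; Collision returns to QueryOnly shortly after that timeline finishes, so grounded overlaps leave it disabled.
; The construction script keeps X and Z, leaving Y at default to flatten placement.
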(event `self.ReceiveActorBeginOverlap`
  (params (OtherActor :type "Actor Object Reference"))
  (bind _ascharacter (cast `Character` OtherActor))
  (`PrimitiveComponent.SetCollisionEnabled` (`self.Collision`) "NoCollision")
  (if (and (`NavMovementComponent.IsFalling` (`Pawn.GetMovementComponent` _ascharacter)) (not (`self.Hit`)))
    (`KismetSystemLibrary.PrintString` "Hello")
    (set `self.Hit` true)
    (bind (_direction _newtrack_0) (`Timeline|Timeline_0` :!via `PlayFromStart`)
      (:`Update`
        (`SceneComponent.K2_SetRelativeLocation` (`self.BlockSprite`) (`KismetMathLibrary.VLerp` (0.0 0.0 0.0) (0.0 0.0 50.0) _newtrack_0) false))
      (:`Finished`
        (set `self.Hit` false)
        (`KismetSystemLibrary.Delay` 0.2)
        (`PrimitiveComponent.SetCollisionEnabled` (`self.Collision`) "QueryOnly")))))

(fn `UserConstructionScript`
  (bind (_returnvalue_x _returnvalue_y _returnvalue_z) (`KismetMathLibrary.BreakVector` (`self.K2_GetActorLocation`)))
  (`self.K2_SetActorLocation` (`KismetMathLibrary.MakeVector` _returnvalue_x 0.0 _returnvalue_z)))