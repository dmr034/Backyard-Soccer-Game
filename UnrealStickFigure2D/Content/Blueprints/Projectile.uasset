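; Fireball projectile actor that damages enemies, drawn with a Paper2D flipbook added in the construction script.
; On BeginPlay it attaches a fireball trail emitter to its TrailAttach component.
; Overlaps with MyCharacter are ignored; any other overlap spawns an ExplodyPuff at the projectile's location and destroys it, first applying DamageAmount if the other actor is an Enemy.
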(event `self.ReceiveBeginPlay`
  (`GameplayStatics.SpawnEmitterAttached` "/Game/Effects/FireballTrail.FireballTrail" (`self.TrailAttach`) "None" (0.0 0.0 0.0) (struct) "SnapToTarget"))

(event `self.ReceiveActorBeginOverlap`
  (params (OtherActor :type "Actor Object Reference"))
  (cast `/Game/Blueprints/MyCharacter` OtherActor
    (:`CastFailed`
      (bind _asenemy (cast `/Game/Blueprints/Enemies/Enemy` OtherActor)
        (:`then`
          (`/Game/Blueprints/Enemies/Enemy.Damage` _asenemy (`self.DamageAmount`)))
        (:`CastFailed`
          _))
      (`|SpawnActorFromClass` "/Game/Blueprints/ExplodyPuff.ExplodyPuff_C" (`KismetMathLibrary.Conv_VectorToTransform` (`self.K2_GetActorLocation`)))
      (`self.K2_DestroyActor`))))

(fn `UserConstructionScript`
  (`AddComponent|PaperFlipbookComponent_58` :`RelativeTransform` (`KismetMathLibrary.MakeTransform` (-30.0 0.0 5.0) (struct) (1.5 1.5 1.5))))