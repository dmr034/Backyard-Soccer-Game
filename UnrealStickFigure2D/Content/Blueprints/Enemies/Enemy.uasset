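; Enemy actor with a 2D sprite that deals fixed damage to MyCharacter on overlap.
; Its Damage event reduces Health, then spawns the KillEnemy emitter and destroys the actor at zero or below.
; The construction script adds the sprite and applies options for lifespan, projectile speed, wave amount and left facing.
; The wavy-motion timeline and sprite-based collision sizing are unconnected, so neither runs.
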(event `self.ReceiveActorBeginOverlap`
  (params (OtherActor :type "Actor Object Reference"))
  (bind _asmy_character (cast `/Game/Blueprints/MyCharacter` OtherActor))
  (`/Game/Blueprints/MyCharacter.Damage` _asmy_character 20.0))

(event `Damage`
  (params (DamageAmount :type "Float (double-precision)" :default 0.0))
  (set `self.Health` (- (`self.Health`) DamageAmount))
  (if (<= (`self.Health`) 0.0)
    (`GameplayStatics.SpawnEmitterAtLocation` "/Game/Effects/KillEnemy.KillEnemy" (`self.K2_GetActorLocation`))
    (`self.K2_DestroyActor`)))

(fn `UserConstructionScript`
  (bind _projectilemovement1 (`self.ProjectileMovement1`))
  (bind _returnvalue (`AddComponent|PaperSpriteComponent_10374`))
  (set `self.Sprite` _returnvalue)
  (`PaperSpriteComponent.SetSprite` _returnvalue (`self.EnemySprite`))
  (if (`self.LiveForever`)
    (`self.SetLifeSpan` 0.0))
  (if (`self.CanAdvance`)
    (set `ProjectileMovementComponent.InitialSpeed` 500.0 _projectilemovement1)
    (else
      (set `ProjectileMovementComponent.InitialSpeed` 0.0 _projectilemovement1)))
  (if (`self.HasWavyMotion`)
    (set `self.InternalWaveAmount` (`self.WaveAmount`))
    (else
      (set `self.InternalWaveAmount` 0.0)))
  (if (`self.FaceLeft`)
    (`SceneComponent.K2_AddRelativeRotation` (`self.Sprite`) (`KismetMathLibrary.MakeRot` 0.0 180.0) false)
    (`self.K2_SetActorLocation` (`KismetMathLibrary.MakeVector` (.x (`self.K2_GetActorLocation`)) 0.0 (.z (`self.K2_GetActorLocation`))))))